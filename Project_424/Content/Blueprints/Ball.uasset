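; Ball actor with a physics-simulated sphere that is pulled or pushed by competing force requests.
; Callers queue normalized direction and distance pairs through AddPotentialForce; each Tick applies only the nearest one as an acceleration scaled by ForceMultiplier, then clears the queue.
; Enable and Disable functions toggle simulation and gravity, with disabling also flagging the ball as interacted.
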(event EventBeginPlay)

(event EventTick
  (params (DeltaSeconds :type Float%20%28single-precision%29))
  (if (and (Physics|IsSimulatingPhysics (Variables|Default|GetSphere) "None") (> (Utilities|Array|Length (Variables|Default|GetPotential%20Forces)) 0))
    (bind _force (CallFunction|GetForce))
    (Physics|AddForce (Variables|Default|GetSphere) (* (.ForceDirection (Utilities|Struct|BreakPotentialForce _force)) (Variables|Default|GetForce%20Multiplier)) "None" true)
    (Utilities|Array|Clear (Variables|Default|GetPotential%20Forces))))

(fn ConstructionScript)

(fn DisablePhysics
  (Physics|SetSimulatePhysics (Variables|Default|GetSphere) false)
  (Physics|SetEnableGravity (Variables|Default|GetSphere) false)
  (Variables|Default|SetbInteracted true))

(fn EnablePhysics
  (Physics|SetSimulatePhysics (Variables|Default|GetSphere) true)
  (Physics|SetEnableGravity (Variables|Default|GetSphere) true))

(fn AddPotentialForce
  (params (Force%20Vector :type Vector) (Distance%20To%20Target :type Float%20%28single-precision%29))
  (Utilities|Array|Add (Variables|Default|GetPotential%20Forces) (Utilities|Struct|MakePotentialForce (Math|Vector|Normalize Force%20Vector) Distance%20To%20Target)))

(fn GetForce
  (if (> (Utilities|Array|Length (Variables|Default|GetPotential%20Forces)) 0)
    (LocalVariables|SetForceToAdd (Utilities|Struct|MakePotentialForce "0.000000,0.000000,0.000000" 1e+05))
    (for _array_element (Variables|Default|GetPotential%20Forces)
      (if (< (.DistanceToTarget (Utilities|Struct|BreakPotentialForce _array_element)) (.DistanceToTarget (Utilities|Struct|BreakPotentialForce (LocalVariables|GetForceToAdd))))
        (LocalVariables|SetForceToAdd _array_element)))
    (return (LocalVariables|GetForceToAdd))
    (else
      (return (Utilities|Struct|MakePotentialForce "0.000000,0.000000,0.000000" 0.0)))))