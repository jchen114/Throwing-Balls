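; Player character that looks around, steers a pivoting hand and uses it to grab, hold and release Ball actors.
; A HandState machine drives timelines that lerp the hand onto an overlapping, recently rendered ball, attach it, then return.
; The grab target inverts the AttachmentPoint offset; releasing retracts a reaching hand or re-enables a held ball's physics.
; Each tick, a camera-forward sphere trace reports hits to SD_Target actors through HitTraceCircle.
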(event EventBeginPlay
  (Variables|Default|SetHand%20State "NewEnumerator0"))

(event Collision|EventActorBeginOverlap
  (params (OtherActor :type Actor%20Object%20Reference)))

(event EventTick
  (params (DeltaSeconds :type Float%20%28single-precision%29))
  (bind _camera (Variables|Default|GetCamera))
  (bind _returnvalue (Transformation|GetWorldLocation _camera))
  (bind _outhits (Collision|MultiSphereTraceByChannel _returnvalue (+ _returnvalue (* (Math|Vector|GetForwardVector (Transformation|GetWorldRotation _camera)) 5e+03)) 1.5e+02 "TraceTypeQuery1" false 0 "None" true "(R=1.000000,G=0.000000,B=0.000000,A=1.000000)" "(R=0.000000,G=1.000000,B=0.000000,A=1.000000)" 0.0))
  (for _array_element _outhits
    (bind _assd_target (Utilities|Casting|CastToSD_Target (.HitActor (Collision|BreakHitResult _array_element))))
    (Default|HitTraceCircle _assd_target (.ImpactPoint (Collision|BreakHitResult _array_element)) (.TraceStart (Collision|BreakHitResult _array_element)) (.TraceEnd (Collision|BreakHitResult _array_element)))))

(event Input|ActionEvents|InputActionGrab/Catch
  (params (Key :type Key%20Structure :default "None"))
  (bind _armsphere (Variables|Default|GetArmSphere))
  (bind _ball (Variables|Default|GetBall))
  (bind _overlappingactors (Collision|GetOverlappingActors _armsphere "/Game/Blueprints/Ball.Ball_C" :!class /Script/Engine.PrimitiveComponent))
  (bind _output (Utilities|Array|Get(acopy) _overlappingactors))
  ;[1 0.982 0] Handle Hand Action
  (:Pressed
    (switch Utilities|FlowControl|Switch|SwitchonEHandState (Variables|Default|GetHand%20State)
      (:NewEnumerator0
        (if (> (Utilities|Array|Length _overlappingactors) 0)
          (if (Class|Actor|WasRecentlyRendered _output 0.0)
            (bind _asball (Utilities|Casting|CastToBall _output))
            (CallFunction|SetupGrabBall _asball)
            ;[0.05951 0.159 0.2542] Move Hand to Ball to grab it
            (bind _grab_alpha (Timeline|Grab%20Timeline PlayFromStart)
              (:Update
                ;;[0 1 0.05568] Move Hand towards Ball
                (switch Utilities|FlowControl|Switch|SwitchonEHandState (Variables|Default|GetHand%20State)
                  (:NewEnumerator1
                    (bind _hand_transform (CallFunction|GetTargetHandTransform (Variables|Default|GetBall)))
                    (Transformation|SetWorldTransform (Variables|Default|GetHand) (Math|Transform|Lerp(Transform) (Transformation|GetWorldTransform (Variables|Default|GetHand)) _hand_transform _grab_alpha) false true))))
              (:Finished
                ;;[1 0 0] Attach Ball to Hand
                (switch Utilities|FlowControl|Switch|SwitchonEHandState (Variables|Default|GetHand%20State)
                  (:NewEnumerator1
                    (Variables|Default|SetHand%20State "NewEnumerator2")
                    (Default|DisablePhysics _ball)
                    (Transformation|AttachComponentToComponent _ball (Variables|Default|GetAttachmentPoint) "None" "KeepWorld" "KeepWorld" "KeepWorld" false)
                    ;;[0.9493 1 0] Return to original position
                    (bind _return_alpha (Timeline|Return%20Timeline PlayFromStart)
                      (:Update
                        (Transformation|SetRelativeTransform (Variables|Default|GetHand) (Math|Transform|Lerp(Transform) (Transformation|GetRelativeTransform (Variables|Default|GetHand)) (Variables|Default|GetPrevious%20Relative%20Hand%20Transform) _return_alpha) false false))))))))))))
  (:Released
    ;[0.05448 0.147 0.2346] Move hand back if releasing while grabbing
    (switch Utilities|FlowControl|Switch|SwitchonEHandState (Variables|Default|GetHand%20State)
      (:NewEnumerator1
        (Variables|Default|SetHand%20State "NewEnumerator3")
        (bind _release_alpha (Timeline|Release%20Timeline PlayFromStart)
          (:Update
            (Transformation|SetRelativeTransform (Variables|Default|GetHand) (Math|Transform|Lerp(Transform) (Transformation|GetRelativeTransform (Variables|Default|GetHand)) (Variables|Default|GetPrevious%20Relative%20Hand%20Transform) _release_alpha) false false))
          (:Finished
            (Variables|Default|SetHand%20State "NewEnumerator0"))))
      (:NewEnumerator2
        ;[0.03415 1 0] Release ball when held
        (Variables|Default|SetHand%20State "NewEnumerator0")
        (Default|EnablePhysics (Variables|Default|GetBall))))))

(event Input|AxisEvents|InputAxisLookUp
  (params (AxisValue :type Float%20%28single-precision%29))
  ;[0 0.1552 1] Handle Camera
  (Transformation|AddLocalRotation (Variables|Default|GetCamera) (Math|Rotator|MakeRotator 0.0 (* AxisValue (Variables|Default|GetDeltaRotation)) 0.0) false false))

(event Input|AxisEvents|InputAxisLookDown
  (params (AxisValue :type Float%20%28single-precision%29))
  ;[0 0.1552 1] Handle Camera
  (Transformation|AddLocalRotation (Variables|Default|GetCamera) (Math|Rotator|MakeRotator 0.0 (* (* AxisValue -1.0) (Variables|Default|GetDeltaRotation)) 0.0) false false))

(event Input|AxisEvents|InputAxisLookRight
  (params (AxisValue :type Float%20%28single-precision%29))
  ;[0 0.1552 1] Handle Camera
  (Transformation|AddLocalRotation (Variables|Default|GetScene) (Math|Rotator|MakeRotator 0.0 0.0 (* AxisValue (Variables|Default|GetDeltaRotation))) false false))

(event Input|AxisEvents|InputAxisLookLeft
  (params (AxisValue :type Float%20%28single-precision%29))
  ;[0 0.1552 1] Handle Camera
  (Transformation|AddLocalRotation (Variables|Default|GetScene) (Math|Rotator|MakeRotator 0.0 0.0 (* (* AxisValue -1.0) (Variables|Default|GetDeltaRotation))) false false))

(event Input|AxisEvents|InputAxisMoveHandLeftRight
  (params (AxisValue :type Float%20%28single-precision%29))
  (bind _pivot (Variables|Default|GetPivot))
  (bind _relativerotation (Variables|/Script/Engine.SceneComponent|GetRelativeRotation _pivot))
  ;[0.1703 1 0.2932] Handle hand movement
  (Transformation|AddRelativeRotation (Variables|Default|GetPivot) (Math|Rotator|MakeRotator 0.0 0.0 AxisValue) false false)
  (Transformation|SetRelativeRotation _pivot (Math|Rotator|MakeRotator (.roll _relativerotation) 0.0 (.yaw _relativerotation)) false false))

(event Input|AxisEvents|InputAxisMoveHandUpDown
  (params (AxisValue :type Float%20%28single-precision%29))
  (bind _pivot (Variables|Default|GetPivot))
  (bind _relativerotation (Variables|/Script/Engine.SceneComponent|GetRelativeRotation _pivot))
  ;[0.1703 1 0.2932] Handle hand movement
  (Transformation|AddRelativeRotation (Variables|Default|GetPivot) (Math|Rotator|MakeRotator AxisValue 0.0 0.0) false false)
  (Transformation|SetRelativeRotation _pivot (Math|Rotator|MakeRotator (.roll _relativerotation) 0.0 (.yaw _relativerotation)) false false))

(fn ConstructionScript)

(fn SetupGrabBall
  (params (Ball :type Ball%20Object%20Reference))
  (Variables|Default|SetPrevious%20Relative%20Hand%20Transform (Transformation|GetRelativeTransform (Variables|Default|GetHand)))
  (Variables|Default|SetHand%20State "NewEnumerator1")
  (Variables|Default|SetBall Ball))

(fn GetTargetHandTransform
  (params (Ball :type Ball%20Object%20Reference))
  (return (Math|Transform|ComposeTransforms (Math|Transform|MakeTransform (Transformation|GetWorldLocation (Variables|/Game/Blueprints/Ball.Ball_C|GetSphere Ball))) (Math|Transform|InvertTransform (Transformation|GetRelativeTransform (Variables|Default|GetAttachmentPoint))))))