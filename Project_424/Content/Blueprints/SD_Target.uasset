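; Target actor that draws Ball actors toward its Person component and spins when a ball hits it.
; Each tick, balls overlapping PullSphere receive a potential force along the horizontal direction to Person, along with their distance to it.
; A ball hit plays the Spin timeline to drive yaw, ignoring further hits until it finishes.
; HitTraceCircle sizes PullSphere by vector projection, shrinking it the farther HitLocation lies from the trace line.
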(event EventBeginPlay)

(event EventTick
  (params (DeltaSeconds :type Float%20%28single-precision%29))
  (for _array_element (Collision|GetOverlappingActors (Variables|Default|GetPull%20Sphere) "/Game/Blueprints/Ball.Ball_C" :!class /Script/Engine.PrimitiveComponent)
    (bind _asball (Utilities|Casting|CastToBall _array_element))
    (Default|AddPotentialForce _asball (Math|Vector|MakeVector (.X (Math|Vector|BreakVector (- (Transformation|GetWorldLocation (Variables|Default|GetPerson)) (Transformation|GetActorLocation _array_element)))) (.Y (Math|Vector|BreakVector (- (Transformation|GetWorldLocation (Variables|Default|GetPerson)) (Transformation|GetActorLocation _array_element)))) 0.0) (Math|Vector|VectorLength (- (Transformation|GetActorLocation _asball) (Transformation|GetWorldLocation (Variables|Default|GetPerson)))))))

(event Collision|EventHit
  (params (MyComp :type Primitive%20Component%20Object%20Reference) (Other :type Actor%20Object%20Reference) (OtherComp :type Primitive%20Component%20Object%20Reference) (bSelfMoved :type Boolean) (HitLocation :type Vector :default "0, 0, 0") (HitNormal :type Vector :default "0, 0, 0") (NormalImpulse :type Vector :default "0, 0, 0") (Hit :type Hit%20Result%20Structure%20%28by%20ref%29))
  (Utilities|Casting|CastToBall Other)
  (if (not (Variables|Default|GetbSpinning))
    (Variables|Default|SetbSpinning true)
    (bind _spin (Timeline|Spin PlayFromStart)
      (:Update
        (Transformation|SetActorRotation (Math|Rotator|MakeRotator 0.0 0.0 (* _spin (Variables|Default|GetSpinningDegrees)))))
      (:Finished
        (Variables|Default|SetbSpinning false)))))

(fn ConstructionScript)

(fn HitTraceCircle
  (params (HitLocation :type Vector) (TraceStart :type Vector) (TraceEnd :type Vector))
  (bind _returnvalue (- HitLocation TraceStart))
  (bind _returnvalue_2 (- TraceEnd TraceStart))
  (bind _returnvalue_3 (Math|Vector|ProjectVectorontoVector _returnvalue _returnvalue_2))
  (LocalVariables|SetProjectedHitVectorOntoTrace _returnvalue_3)
  (LocalVariables|SetNormalVectorFromTrace (- _returnvalue _returnvalue_3))
  (Utilities|FlowControl|Sequence
    (:then_0
      (Components|Sphere|SetSphereRadius (Variables|Default|GetPull%20Sphere) (- (Variables|Default|GetRadius) (Math|Vector|VectorLength (LocalVariables|GetNormalVectorFromTrace))) true))))